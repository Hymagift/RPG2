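; BP_Pnj is a damageable NPC character with an overhead health bar widget and a ragdoll death.
; Any damage plays a random hit-react montage, launches it along the player's facing direction and lowers health through BPCPlayerStats.
; When DecreaseHealth returns true, the mesh simulates physics and the health bar hides.
; Tick rotates the bar toward the camera, though the look-at starts from its forward vector instead of its location.
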(event EventBeginPlay
  (Utilities|FlowControl|DelayUntilNextTick)
  (bind _aswp_pnjhealth_bar (Utilities|Casting|CastToWp_PNJHealthBar (UserInterface|GetWidget (Variables|Default|GethealthBar))))
  (Variables|Default|SetHealthBarWidget _aswp_pnjhealth_bar))

(event Collision|EventActorBeginOverlap
  (params (OtherActor :type Actor%20Object%20Reference)))

(event EventTick
  (params (DeltaSeconds :type Float%20%28single-precision%29))
  (Transformation|SetWorldRotation (Variables|Default|GethealthBar) (Math|Rotator|FindLookatRotation (Math|Rotator|GetRotationXVector (Transformation|GetWorldRotation (Variables|Default|GethealthBar))) (Camera|GetCameraLocation (Game|GetPlayerCameraManager 0))) false false))

(event Game|Damage|EventAnyDamage
  (params (Damage :type Float%20%28single-precision%29) (DamageType :type Damage%20Type%20Object%20Reference) (InstigatedBy :type Controller%20Object%20Reference) (DamageCauser :type Actor%20Object%20Reference))
  (Animation|PlayAnimMontage (Utilities|Array|Get(acopy) (Variables|Default|GetHitReact) (Math|Random|RandomIntegerinRange 0 (- (Utilities|Array|Length (Variables|Default|GetHitReact)) 1))) 1.0 "None")
  (bind _asbp_third_person_character (Utilities|Casting|CastToBP_ThirdPersonCharacter (Game|GetPlayerCharacter 0))
    (:then
      (Character|LaunchCharacter (* (Math|Vector|GetForwardVector (Transformation|GetActorRotation _asbp_third_person_character)) 7e+02) false false)
      (bind _isdead (Default|DecreaseHealth (Variables|Default|GetBPC_PlayerStats) Damage))
      (if _isdead
        (Physics|SetSimulatePhysics (Variables|Character|GetMesh) true)
        (Rendering|SetVisibility (Variables|Default|GethealthBar) false false)))
    (:CastFailed
      (Development|PrintString "Hello"))))

(fn ConstructionScript)