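; Player attack component for the third-person character: runs a four-step sword and kick combo from the attack input and deals damage through traces.
; An enum picks each montage and advances when it plays, while input during an attack buffers the next step for SwordAttackCombo, otherwise the combo resets.
; A looping timer sweeps sphere traces along the blade against PNJ-tagged actors, and a separate point trace hits Damagable-tagged ones, both adding camera shake.
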(event Custom|Swordattack
  ;[0.15 0.15 0.15 0.5] Attack
  (if (Variables|Default|GetIsAttacking)
    (Variables|Default|SetSaveAttack true)
    (else
      (Variables|Default|SetIsAttacking true)
      (switch Utilities|FlowControl|Switch|SwitchonAttackEnum (Variables|Default|GetAttackEnum)
        (:NewEnumerator0
          (CallFunction|Attack1))
        (:NewEnumerator1
          (CallFunction|Attack2))
        (:NewEnumerator3
          (CallFunction|Attack3))
        (:NewEnumerator2
          (CallFunction|Attack4))))))

(event Custom|SwordAttackCombo
  ;[0.15 0.15 0.15 0.5] Attack
  (if (Variables|Default|GetSaveAttack)
    (Variables|Default|SetSaveAttack false)
    (switch Utilities|FlowControl|Switch|SwitchonAttackEnum (Variables|Default|GetAttackEnum)
      (:NewEnumerator0
        (CallFunction|Attack1))
      (:NewEnumerator1
        (CallFunction|Attack2))
      (:NewEnumerator3
        (CallFunction|Attack3))
      (:NewEnumerator2
        (CallFunction|Attack4)))
    (else
      (CallFunction|StopCombo))))

(event Custom|StopSwordTrace
  ;[0.15 0.15 0.15 0.5] SwordTrace
  (Utilities|Time|ClearandInvalidateTimerbyHandle (Variables|Default|GetSwordTraceLoop)))

(event Custom|SwordTrace
  ;[0.15 0.15 0.15 0.5] SwordTrace
  (bind (_outhit _returnvalue) (Collision|SphereTraceByChannel (Transformation|GetWorldLocation (Variables|/Game/ThirdPerson/Blueprints/BP_ThirdPersonCharacter.BP_ThirdPersonCharacter_C|GetSwordTopPoint (Variables|Default|GetCharacterBP))) (Transformation|GetWorldLocation (Variables|/Game/ThirdPerson/Blueprints/BP_ThirdPersonCharacter.BP_ThirdPersonCharacter_C|GetSwordBottomPoint (Variables|Default|GetCharacterBP))) 12.0 "TraceTypeQuery1" false 0 "None" true "(R=1.000000,G=0.000000,B=0.000000,A=1.000000)" "(R=0.000000,G=1.000000,B=0.000000,A=1.000000)" 0.3))
  (if _returnvalue
    (if (Actor|ActorHasTag (.HitActor (Collision|BreakHitResult _outhit)) "PNJ")
      (Utilities|FlowControl|DoOnce false :!label _label
        (:Completed
          (Game|Damage|ApplyDamage (.HitActor (Collision|BreakHitResult _outhit)) 1e+01 0 0)
          (Camera|PlayWorldCameraShake "/Game/10_Blueprints/10_Animations/BP_CameraShake.BP_CameraShake_C" (.Location (Collision|BreakHitResult _outhit)) 0.0 2e+03)
          (Utilities|FlowControl|Delay 0.5)
          (goto _label Reset))))))

(event Custom|SphereTrace
  (bind _characterbp (Variables|Default|GetCharacterBP))
  (bind _spheretrace (Variables|/Game/ThirdPerson/Blueprints/BP_ThirdPersonCharacter.BP_ThirdPersonCharacter_C|GetSphereTrace _characterbp))
  (bind _returnvalue (Transformation|GetWorldLocation _spheretrace))
  ;[0.15 0.15 0.15 0.5] SphereTraceEstocAndKick
  (bind (_outhit _returnvalue_2) (Collision|SphereTraceByChannel _returnvalue _returnvalue 25.0 "TraceTypeQuery1" false 0 "None" true "(R=1.000000,G=0.000000,B=0.000000,A=1.000000)" "(R=0.000000,G=1.000000,B=0.000000,A=1.000000)" 0.001))
  (if _returnvalue_2
    (if (Actor|ActorHasTag (.HitActor (Collision|BreakHitResult _outhit)) "Damagable")
      (Game|Damage|ApplyDamage (.HitActor (Collision|BreakHitResult _outhit)) 1e+01 0 0)
      (Camera|PlayWorldCameraShake "/Game/10_Blueprints/10_Animations/BP_CameraShake.BP_CameraShake_C" (.Location (Collision|BreakHitResult _outhit)) 0.0 2e+03))))

(event Custom|StopCombo
  ;[0.15 0.15 0.15 0.5] Attack
  (Variables|Default|SetIsAttacking false)
  (Variables|Default|SetAttackEnum "NewEnumerator0"))

(event Custom|Attack4
  ;[0.15 0.15 0.15 0.5] Attack
  (Utilities|FlowControl|DoOnce false :!label _label
    (:Completed
      (Utilities|FlowControl|Delay 0.1)
      (Animation|Montage|PlayMontage (Variables|Default|GetCharacterMesh) "/Game/20_Animations/SwordAttacks/Attack3_Montage.Attack3_Montage"
        (:then
          (Variables|Default|SetAttackEnum "NewEnumerator0")
          (goto _label Reset))))))

(event Custom|Attack1
  ;[0.15 0.15 0.15 0.5] Attack
  (Utilities|FlowControl|DoOnce false :!label _label
    (:Completed
      (Utilities|FlowControl|Delay 0.1)
      (Animation|Montage|PlayMontage (Variables|Default|GetCharacterMesh) "/Game/20_Animations/SwordAttacks/Attack1_Montage.Attack1_Montage"
        (:then
          (Variables|Default|SetAttackEnum "NewEnumerator1")
          (goto _label Reset))))))

(event Custom|Start%20SwordTrace
  ;[0.15 0.15 0.15 0.5] SwordTrace
  (bind _returnvalue (Utilities|Time|SetTimerbyEvent (delegate Custom|SwordTrace) 0.001 true))
  (Variables|Default|SetSwordTraceLoop _returnvalue))

(event Custom|Attack2
  ;[0.15 0.15 0.15 0.5] Attack
  (Utilities|FlowControl|DoOnce false :!label _label
    (:Completed
      (Utilities|FlowControl|Delay 0.1)
      (Animation|Montage|PlayMontage (Variables|Default|GetCharacterMesh) "/Game/20_Animations/SwordAttacks/Attack2_Montage.Attack2_Montage"
        (:then
          (Variables|Default|SetAttackEnum "NewEnumerator3")
          (goto _label Reset))))))

(event Custom|Attack3
  ;[0.15 0.15 0.15 0.5] Attack
  (Utilities|FlowControl|DoOnce false :!label _label
    (:Completed
      (Utilities|FlowControl|Delay 0.1)
      (Animation|Montage|PlayMontage (Variables|Default|GetCharacterMesh) "/Game/20_Animations/SwordAttacks/Kick_Montage.Kick_Montage"
        (:then
          (Variables|Default|SetAttackEnum "NewEnumerator2")
          (goto _label Reset))))))

(event Input|EnhancedActionEvents|EnhancedInputActionIA_Attack
  (params (ActionValue :type Boolean) (ElapsedSeconds :type Float%20%28double-precision%29) (TriggeredSeconds :type Float%20%28double-precision%29) (InputAction :type Input%20Action%20Object%20Reference :default "/Game/Input/Actions/IA_Attack.IA_Attack"))
  ;[0.15 0.15 0.15 0.5] Attack
  (:Started
    (if (Variables|Default|GetCanAttack)
      (CallFunction|Swordattack))))

(event EventBeginPlay
  ;[0.15 0.15 0.15 0.5] Attack
  (bind _asbp_third_person_character (Utilities|Casting|CastToBP_ThirdPersonCharacter (Components|GetOwner)))
  (Variables|Default|SetCharacterBP _asbp_third_person_character)
  (Variables|Default|SetCharacterMesh (Variables|/Script/Engine.Character|GetMesh _asbp_third_person_character)))