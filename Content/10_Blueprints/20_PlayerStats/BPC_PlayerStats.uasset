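; Actor component that tracks health and stamina for the player character or an NPC (BP_Pnj) and drives their UI.
; One tick after BeginPlay it identifies its owner and initializes the health display.
; Functions change current or maximum values and refresh widgets directly, with decrease functions returning true on depletion.
; Only initialization and DecreaseHealth support NPC health bars; other functions write straight to the player widget.
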(event EventBeginPlay
  (Utilities|FlowControl|DelayUntilNextTick)
  (bind _asbp_third_person_character (Utilities|Casting|CastToBP_ThirdPersonCharacter (Components|GetOwner))
    (:then
      (Variables|Default|SetCharacter _asbp_third_person_character)
      (Variables|Default|SetIsPlayer true))
    (:CastFailed
      (bind _asbp_pnj (Utilities|Casting|CastToBP_Pnj (Components|GetOwner)))
      (Variables|Default|SetBP_Pnj _asbp_pnj)
      (Variables|Default|SetIsPlayer false)))
  (Progress|SetPercent (Variables|/Game/30_UI/BP_HUD.BP_HUD_C|GetHpBar (Variables|/Game/ThirdPerson/Blueprints/BP_ThirdPersonCharacter.BP_ThirdPersonCharacter_C|GetWidget (Variables|Default|GetCharacter))) (/ (Variables|Health|GetCurrentHealth) (Variables|Health|GetMaxHealth)))
  (Rendering|Components|TextRender|SetText (select (Variables|Default|GetIsPlayer) (Variables|/Game/30_UI/BP_HUD.BP_HUD_C|GetHealthText (Variables|/Game/ThirdPerson/Blueprints/BP_ThirdPersonCharacter.BP_ThirdPersonCharacter_C|GetWidget (Variables|Default|GetCharacter))) (Variables|/Game/10_Blueprints/40_PNJ/Wp_PNJHealthBar.Wp_PNJHealthBar_C|GetHealthText (Variables|/Game/10_Blueprints/40_PNJ/BP_Pnj.BP_Pnj_C|GetHealthBarWidget (Variables|Default|GetBP_Pnj)))) (Utilities|Text|ToText(Float) (Variables|Health|GetCurrentHealth) "HalfToEven")))

(fn DecreaseHealth
  (params (DamageAmount :type Float%20%28double-precision%29))
  (bind _character (Variables|Default|GetCharacter))
  (bind _widget (Variables|/Game/ThirdPerson/Blueprints/BP_ThirdPersonCharacter.BP_ThirdPersonCharacter_C|GetWidget _character))
  (if (not (<= (Variables|Health|GetCurrentHealth) 0.0))
    (bind _output_get (Variables|Health|SetCurrentHealth (- (Variables|Health|GetCurrentHealth) DamageAmount)))
    (Progress|SetPercent (select (Variables|Default|GetIsPlayer) (Variables|/Game/30_UI/BP_HUD.BP_HUD_C|GetHpBar _widget) (Variables|/Game/10_Blueprints/40_PNJ/Wp_PNJHealthBar.Wp_PNJHealthBar_C|GetHealthBar (Variables|/Game/10_Blueprints/40_PNJ/BP_Pnj.BP_Pnj_C|GetHealthBarWidget (Variables|Default|GetBP_Pnj)))) (/ _output_get (Variables|Health|GetMaxHealth)))
    (Rendering|Components|TextRender|SetText (select (Variables|Default|GetIsPlayer) (Variables|/Game/30_UI/BP_HUD.BP_HUD_C|GetHealthText _widget) (Variables|/Game/10_Blueprints/40_PNJ/Wp_PNJHealthBar.Wp_PNJHealthBar_C|GetHealthText (Variables|/Game/10_Blueprints/40_PNJ/BP_Pnj.BP_Pnj_C|GetHealthBarWidget (Variables|Default|GetBP_Pnj)))) (Utilities|Text|ToText(Float) (Variables|Health|GetCurrentHealth) "HalfToEven"))
    (if (<= (Variables|Health|GetCurrentHealth) 0.0)
      _
      (else
        (return false))))
  (return true))

(fn IncreaseMaxHealth
  (params (HPGained :type Float%20%28double-precision%29))
  (bind _character (Variables|Default|GetCharacter))
  (bind _widget (Variables|/Game/ThirdPerson/Blueprints/BP_ThirdPersonCharacter.BP_ThirdPersonCharacter_C|GetWidget _character))
  (Variables|Health|SetMaxHealth (+ (Variables|Health|GetMaxHealth) HPGained))
  (Progress|SetPercent (Variables|/Game/30_UI/BP_HUD.BP_HUD_C|GetHpBar _widget) (/ (Variables|Health|GetCurrentHealth) (Variables|Health|GetMaxHealth)))
  (Variables|/Script/UMG.TextBlock|SetText (Variables|/Game/30_UI/BP_HUD.BP_HUD_C|GetHealthText _widget) (Utilities|Text|ToText(Float) (Variables|Health|GetCurrentHealth) "HalfToEven")))

(fn DecreaseStamina
  (params (StaminaLost :type Float%20%28double-precision%29))
  (if (not (<= (Variables|Endurance|GetCurrentStamina) 0.0))
    (Variables|Endurance|SetCurrentStamina (- (Variables|Endurance|GetCurrentStamina) StaminaLost))
    (Progress|SetPercent (Variables|/Game/30_UI/BP_HUD.BP_HUD_C|GetStamina (Variables|/Game/ThirdPerson/Blueprints/BP_ThirdPersonCharacter.BP_ThirdPersonCharacter_C|GetWidget (Variables|Default|GetCharacter))) (/ (Variables|Endurance|GetCurrentStamina) (Variables|Endurance|GetMaxStamina)))
    (if (<= (Variables|Endurance|GetCurrentStamina) 0.0)
      _
      (else
        (return false))))
  (return true))

(fn IncreaseMaxStamina
  (params (StaminaGained :type Float%20%28double-precision%29))
  (Variables|Endurance|SetMaxStamina (+ (Variables|Endurance|GetMaxStamina) StaminaGained))
  (Progress|SetPercent (Variables|/Game/30_UI/BP_HUD.BP_HUD_C|GetStamina (Variables|/Game/ThirdPerson/Blueprints/BP_ThirdPersonCharacter.BP_ThirdPersonCharacter_C|GetWidget (Variables|Default|GetCharacter))) (/ (Variables|Endurance|GetCurrentStamina) (Variables|Endurance|GetMaxStamina))))

(fn IncreaseHealth
  (params (AddedHealth :type Float%20%28double-precision%29))
  (bind _character (Variables|Default|GetCharacter))
  (bind _widget (Variables|/Game/ThirdPerson/Blueprints/BP_ThirdPersonCharacter.BP_ThirdPersonCharacter_C|GetWidget _character))
  (Variables|Health|SetCurrentHealth (+ (Variables|Health|GetCurrentHealth) AddedHealth))
  (if (> (Variables|Health|GetCurrentHealth) (Variables|Health|GetMaxHealth))
    (Variables|Health|SetCurrentHealth (Variables|Health|GetMaxHealth)))
  (Progress|SetPercent (Variables|/Game/30_UI/BP_HUD.BP_HUD_C|GetHpBar _widget) (/ (Variables|Health|GetCurrentHealth) (Variables|Health|GetMaxHealth)))
  (Variables|/Script/UMG.TextBlock|SetText (Variables|/Game/30_UI/BP_HUD.BP_HUD_C|GetHealthText _widget) (Utilities|Text|ToText(Float) (Variables|Health|GetCurrentHealth) "HalfToEven")))

(fn IncreaseStamina
  (params (AddedStamina :type Float%20%28double-precision%29))
  (Variables|Endurance|SetCurrentStamina (+ (Variables|Endurance|GetCurrentStamina) AddedStamina))
  (if (> (Variables|Endurance|GetCurrentStamina) (Variables|Endurance|GetMaxStamina))
    (Variables|Endurance|SetCurrentStamina (Variables|Endurance|GetMaxStamina)))
  (Progress|SetPercent (Variables|/Game/30_UI/BP_HUD.BP_HUD_C|GetStamina (Variables|/Game/ThirdPerson/Blueprints/BP_ThirdPersonCharacter.BP_ThirdPersonCharacter_C|GetWidget (Variables|Default|GetCharacter))) (/ (Variables|Endurance|GetCurrentStamina) (Variables|Endurance|GetMaxStamina))))